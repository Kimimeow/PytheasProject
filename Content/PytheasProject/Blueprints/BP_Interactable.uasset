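; BP_Interactable is an interactable actor that shows dialogue text on screen.
; Its Interact event toggles a WBP_Dialogue widget, either creating it for player 0 and passing in DialogueText, or removing the existing one.
; When BP_Player leaves the Box trigger, the widget is removed and its reference cleared, without a validity check.
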(event OnComponentEndOverlap(Box)
  (params (OverlappedComponent :type Primitive%20Component%20Object%20Reference) (OtherActor :type Actor%20Object%20Reference) (OtherComp :type Primitive%20Component%20Object%20Reference) (OtherBodyIndex :type Integer))
  (Utilities|Casting|CastToBP_Player OtherActor)
  (Widget|RemovefromParent (Variables|Dialogue|GetDialogueWidget))
  (Variables|Dialogue|SetDialogueWidget 0))

(event EventInteract
  (Utilities|IsValid (Variables|Dialogue|GetDialogueWidget)
    (:Is%20Valid
      (Widget|RemovefromParent (Variables|Dialogue|GetDialogueWidget))
      (Variables|Dialogue|SetDialogueWidget 0))
    (:Is%20Not%20Valid
      (bind _returnvalue (UserInterface|CreateWidget "/Game/PytheasProject/Blueprints/Dialogue/WBP_Dialogue.WBP_Dialogue_C" (Game|GetPlayerController 0)))
      (bind _output_get (Variables|Dialogue|SetDialogueWidget _returnvalue))
      (UserInterface|Viewport|AddtoViewport _output_get 0)
      (Variables|/Game/PytheasProject/Blueprints/Dialogue/WBP_Dialogue.WBP_Dialogue_C|SetDialogue (Variables|Dialogue|GetDialogueWidget) (Variables|Dialogue|GetDialogueText)))))

(fn ConstructionScript)