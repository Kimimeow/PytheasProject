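; BP_NPC is an interactable character that plays sequential dialogue from the Dialogue data table.
; On BeginPlay it collects the rows matching its NPCID.
; Each Interact advances the line counter, shows the line matching the ConversationID in a WBP_Dialogue widget, and yaws the NPC toward the player.
; An empty line closes the widget and resets the counter; the player leaving the Box removes the widget without resetting it.
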(event OnComponentEndOverlap(Box)
  (params (OverlappedComponent :type Primitive%20Component%20Object%20Reference) (OtherActor :type Actor%20Object%20Reference) (OtherComp :type Primitive%20Component%20Object%20Reference) (OtherBodyIndex :type Integer))
  ;[1 1 1] End Dialogue when character moves away
  (Utilities|Casting|CastToBP_Player OtherActor)
  (Widget|RemovefromParent (Variables|Default|GetDialogueWidget))
  (Variables|Default|SetDialogueWidget 0))

(event EventBeginPlay
  ;[1 1 1] Get Characters Dialogue Options
  (bind _outrownames (DataTable|GetDataTableRowNames "/Game/PytheasProject/Blueprints/Dialogue/Dialogue.Dialogue"))
  (for _array_element _outrownames
    (bind _returnvalue (Utilities|GetDataTableRow "/Game/PytheasProject/Blueprints/Dialogue/Dialogue.Dialogue" _array_element)
      (:then
        (if (== (.NPC_ID (Utilities|Struct|BreakDialogueStructure _returnvalue)) (Variables|Default|GetNPC_ID))
          (Utilities|Array|Add (Variables|Default|GetDialogue) _array_element))))))

(event EventInteract
  ;[1 1 1] Set Dialogue Sequence Number
  (Math|Integer|IncrementInt (Variables|Default|GetLineCurrent)
    (:%20%20
      (CallFunction|DialogueCreate)
      ;[1 1 1] Look at Player Character
      (Transformation|SetActorRotation (Math|Rotator|MakeRotator 0.0 0.0 (.yaw (Math|Rotator|FindLookatRotation (Transformation|GetActorLocation) (Transformation|GetActorLocation (Game|GetPlayerCharacter 0)))))))))

(fn ConstructionScript)

(fn DialogueCreate
  (Utilities|IsValid (Variables|Default|GetDialogueWidget)
    (:Is%20Valid
      _)
    (:Is%20Not%20Valid
      (bind _returnvalue (UserInterface|CreateWidget "/Game/PytheasProject/Blueprints/Dialogue/WBP_Dialogue.WBP_Dialogue_C" (Game|GetPlayerController 0)))
      (bind _output_get (Variables|Default|SetDialogueWidget _returnvalue))
      (UserInterface|Viewport|AddtoViewport _output_get 0)))
  (bind _returnedline (CallFunction|DialogueGetLine))
  (if (Utilities|Enum|NotEqual(Enum) _returnedline (Class|KismetTextLibrary|GetEmptyText))
    (Variables|/Game/PytheasProject/Blueprints/Dialogue/WBP_Dialogue.WBP_Dialogue_C|SetDialogue (Variables|Default|GetDialogueWidget) _returnedline)
    (else
      (Widget|RemovefromParent (Variables|Default|GetDialogueWidget))
      (Variables|Default|SetDialogueWidget 0)
      (Variables|Default|SetLineCurrent 0))))

(fn DialogueGetLine
  (for _array_element (Variables|Default|GetDialogue)
    (bind _returnvalue (Utilities|GetDataTableRow "/Game/PytheasProject/Blueprints/Dialogue/Dialogue.Dialogue" _array_element)
      (:then
        (if (and (== (.Conversation_ID (Utilities|Struct|BreakDialogueStructure _returnvalue)) (Variables|Default|GetConversation_ID)) (== (.Line_ID (Utilities|Struct|BreakDialogueStructure _returnvalue)) (Variables|Default|GetLineCurrent)))
          (Utilities|Array|Add (LocalVariables|GetReturnedLines) (.Dialogue (Utilities|Struct|BreakDialogueStructure _returnvalue)))))))
  (if (== (Utilities|Array|Length (LocalVariables|GetReturnedLines)) 1)
    (return (Utilities|Array|Get(acopy) (LocalVariables|GetReturnedLines)))))