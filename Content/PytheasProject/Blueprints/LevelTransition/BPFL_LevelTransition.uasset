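; Blueprint function library for level transitions and per-level startup.
; PlayTransition creates a black or white fade widget, chosen by a color value, plays it in the given play mode and adds it to the viewport.
; SetupLevel fades in the level's ambience and music, then creates the main UI widget for the first player, configured with avatar, year and a void flag.
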(fn PlayTransition
  (params (Transition :type ETransitionEffect%20Enum :default "NewEnumerator0") (PlayMode :type EUMGSequencePlayMode%20Enum :default "Forward") (Color :type Integer))
  (LocalVariables|SetPlay%20Mode PlayMode)
  (switch Utilities|FlowControl|Switch|SwitchonETransitionEffect Transition
    (:NewEnumerator1
      (switch int Color
        (:0
          (bind _returnvalue (UserInterface|CreateWidget "/Game/PytheasProject/Blueprints/LevelTransition/WBP_Level_FadeInOut_Black.WBP_Level_FadeInOut_Black_C"))
          (Default|PlayTransition _returnvalue (LocalVariables|GetPlay%20Mode))
          (UserInterface|Viewport|AddtoViewport _returnvalue 0))
        (:1
          (bind _returnvalue_2 (UserInterface|CreateWidget "/Game/PytheasProject/Blueprints/LevelTransition/WBP_Level_FadeInOut_White.WBP_Level_FadeInOut_White_C"))
          (Default|PlayTransition _returnvalue_2 (LocalVariables|GetPlay%20Mode))
          (UserInterface|Viewport|AddtoViewport _returnvalue_2 0))))))

(fn SetupLevel
  (params (isVoid :type Boolean) (Avatar :type Integer) (Year :type Text) (LevelMusic :type Audio%20Component%20Object%20Reference) (LevelAmbience :type Audio%20Component%20Object%20Reference))
  ;[1 1 1] Start Music on Load
  (Audio|Components|Audio|FadeIn LevelAmbience 1.0 1.0 0.0 "Logarithmic" :!class /Script/Engine.AudioComponent)
  (Audio|Components|Audio|FadeIn LevelMusic 3.0 1.0 0.0 "Linear" :!class /Script/Engine.AudioComponent)
  (bind _returnvalue (UserInterface|CreateWidget "/Game/PytheasProject/Blueprints/UI/WBP_UI.WBP_UI_C" (Game|GetPlayerController 0)))
  (Default|SetupUI _returnvalue Avatar Year isVoid)
  (UserInterface|Viewport|AddtoViewport _returnvalue 0))