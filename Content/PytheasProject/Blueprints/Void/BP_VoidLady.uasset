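; BP_VoidLady is an interactable NPC that the player can start a dialogue with.
; On BeginPlay it hands its DialogueTree to BP_LadyAIController, which starts the conversation when Interact fires.
; A collision volume shows the prompt widget when the player approaches, and on exit hides it and clears the player's InteractionActive flag.
; Interacting also hides the prompt and blends the view to a dialogue camera.
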(event OnComponentBeginOverlap(Collision)
  (params (OverlappedComponent :type Primitive%20Component%20Object%20Reference) (OtherActor :type Actor%20Object%20Reference) (OtherComp :type Primitive%20Component%20Object%20Reference) (OtherBodyIndex :type Integer) (bFromSweep :type Boolean) (SweepResult :type Hit%20Result%20Structure%20%28by%20ref%29))
  ;[1 1 1] Make interaction prompt visible when character is close enough
  (bind _asbp_player (Utilities|Casting|CastToBP_Player OtherActor))
  (if (not (Variables|/Game/PytheasProject/Blueprints/BP_Player.BP_Player_C|GetInteractionActive _asbp_player))
    (Rendering|SetVisibility (Variables|Default|GetWidgetPrompt) true false)))

(event OnComponentEndOverlap(Collision)
  (params (OverlappedComponent :type Primitive%20Component%20Object%20Reference) (OtherActor :type Actor%20Object%20Reference) (OtherComp :type Primitive%20Component%20Object%20Reference) (OtherBodyIndex :type Integer))
  ;[1 1 1] End Dialogue when character moves away
  (bind _asbp_player (Utilities|Casting|CastToBP_Player OtherActor))
  (Variables|/Game/PytheasProject/Blueprints/BP_Player.BP_Player_C|SetInteractionActive _asbp_player false)
  (Rendering|SetVisibility (Variables|Default|GetWidgetPrompt) false false))

(event EventBeginPlay
  ;[1 1 1] Setup Widgets
  (Rendering|SetVisibility (Variables|Default|GetWidgetPrompt) false false)
  ;[1 1 1] Get AI controller and set Dialogue Tree
  (bind _asbp_lady_aicontroller (Utilities|Casting|CastToBP_LadyAIController (AI|GetAIController self)))
  (Variables|/Game/PytheasProject/Blueprints/Void/BP_LadyAIController.BP_LadyAIController_C|SetDialogueTree _asbp_lady_aicontroller (Variables|Default|GetDialogueTree)))

(event EventInteract
  ;[1 1 1] Start Dialogue
  (bind _asbp_lady_aicontroller (Utilities|Casting|CastToBP_LadyAIController (AI|GetAIController self)))
  (Default|StartDialogue _asbp_lady_aicontroller)
  (Rendering|SetVisibility (Variables|Default|GetWidgetPrompt) false false)
  (Game|Player|SetViewTargetwithBlend (Game|GetPlayerController 0) (Variables|Default|GetDialogueCamera) 0.5 "VTBlend_Linear" 0.0 false))

(fn ConstructionScript)