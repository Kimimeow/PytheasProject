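; Behavior tree task that opens the dialogue choice UI when the Void Lady AI starts a conversation.
; It shows the game mode's ChoiceHUD dialogue widget, sets its name from the Void Lady pawn and stores the widget in a blackboard key for later use.
; It then disables player input and finishes successfully.
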(event EventReceiveExecuteAI
  (params (OwnerController :type AI%20Controller%20Object%20Reference) (ControlledPawn :type Pawn%20Object%20Reference))
  (bind _asbp_void_lady (Utilities|Casting|CastToBP_VoidLady ControlledPawn))
  (Variables|Default|SetVoidLadyPawn _asbp_void_lady)
  (bind _asadventure_game_mode (Utilities|Casting|CastToAdventureGameMode (Game|GetGameMode)))
  (Widget|SetVisibility (Variables|/Game/PytheasProject/Blueprints/Void/WBP_ChoiceHUD.WBP_ChoiceHUD_C|GetWBP_DialogueChoice (Variables|/Game/PytheasProject/Blueprints/AdventureGameMode.AdventureGameMode_C|GetChoiceHUD _asadventure_game_mode)) "Visible")
  (Variables|/Game/PytheasProject/Blueprints/Void/WBP_DialogueChoice.WBP_DialogueChoice_C|SetName (Variables|/Game/PytheasProject/Blueprints/Void/WBP_ChoiceHUD.WBP_ChoiceHUD_C|GetWBP_DialogueChoice (Variables|/Game/PytheasProject/Blueprints/AdventureGameMode.AdventureGameMode_C|GetChoiceHUD _asadventure_game_mode)) (Variables|/Game/PytheasProject/Blueprints/Void/BP_VoidLady.BP_VoidLady_C|GetName (Variables|Default|GetVoidLadyPawn)))
  (Class|BTFunctionLibrary|SetBlackboardValueasObject (Variables|Default|GetBB_DialogueUI) (Variables|/Game/PytheasProject/Blueprints/Void/WBP_ChoiceHUD.WBP_ChoiceHUD_C|GetWBP_DialogueChoice (Variables|/Game/PytheasProject/Blueprints/AdventureGameMode.AdventureGameMode_C|GetChoiceHUD _asadventure_game_mode)))
  (Input|DisableInput (Game|GetPlayerCharacter 0) (Game|GetPlayerController 0))
  (AI|BehaviorTree|FinishExecute true))