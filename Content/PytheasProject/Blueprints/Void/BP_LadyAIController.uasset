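; AI controller for the Lady character that drives her dialogue logic through behavior trees.
; StartDialogue calls ChooseTree, which switches on the game instance's LevelID, converted to a string, to run one of three trees (BT_V0, BT_Q1, BT_Q2).
; EndDialogue stops the brain component's logic.
; An older VoidNum counter that stepped through the trees remains in ChooseTree but is disconnected.
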(event Custom|StartDialogue
  (CallFunction|ChooseTree))

(event Custom|EndDialogue
  (AI|Logic|StopLogic (Variables|Default|GetBrainComponent) ""))

(fn ConstructionScript)

(fn ChooseTree
  (bind _asadventure_game_instance (Utilities|Casting|CastToAdventureGameInstance (Game|GetGameInstance)))
  (switch string (Utilities|String|ToString(Integer) (Variables|/Game/PytheasProject/Blueprints/AdventureGameInstance.AdventureGameInstance_C|GetLevelID _asadventure_game_instance))
    (:0
      (bind _output_get (Variables|Default|SetTree "/Game/PytheasProject/Blueprints/Void/BT_V0.BT_V0"))
      (AI|RunBehaviorTree _output_get))
    (:9
      (bind _output_get_2 (Variables|Default|SetTree "/Game/PytheasProject/Blueprints/Void/BT_Q1.BT_Q1"))
      (AI|RunBehaviorTree _output_get_2))
    (:21
      (bind _output_get_3 (Variables|Default|SetTree "/Game/PytheasProject/Blueprints/Void/BT_Q2.BT_Q2"))
      (AI|RunBehaviorTree _output_get_3))))