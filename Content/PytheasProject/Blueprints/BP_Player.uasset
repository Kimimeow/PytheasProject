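; Player character for a point-and-click adventure, handling cursor-driven movement and dialogue interaction.
; BeginPlay enables the mouse cursor with Game and UI input and caches the ChoiceHUD from AdventureGameMode.
; Each Move press checks all BPI_Dialogue actors for overlap, toggling InteractionActive and, on activation, sending InteractMessage and halting movement.
; While no interaction is active, it turns the control rotation toward the clicked point and paths there via SimpleMoveToLocation.
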(event EventBeginPlay
  (Input|SetInputModeGameandUI (Game|GetPlayerController 0) 0 "DoNotLock" true)
  ;[1 1 1] Enable Mouse Cursor
  (Variables|/Script/Engine.PlayerController|SetbShowMouseCursor (Game|GetPlayerController 0) true)
  ;[1 1 1] Get reference to Dialogue HUD for choices
  (bind _asadventure_game_mode (Utilities|Casting|CastToAdventureGameMode (Game|GetGameMode)))
  (Variables|Default|SetChoice%20HUD (Variables|/Game/PytheasProject/Blueprints/AdventureGameMode.AdventureGameMode_C|GetChoiceHUD _asadventure_game_mode)))

(event Input|ActionEvents|InputActionMove
  (params (Key :type Key%20Structure :default "None"))
  (bind _returnvalue (Game|GetPlayerController 0))
  (bind _hitresult (Game|Player|GetHitResultUnderCursorbyChannel _returnvalue "TraceTypeQuery1" true))
  ;[1 1 1] Interact with Characters and Objects
  (:Pressed
    (bind _outactors (Actor|GetAllActorswithInterface "/Game/PytheasProject/Blueprints/Dialogue/BPI_Dialogue.BPI_Dialogue_C"))
    (for _array_element _outactors
      (if (Collision|IsOverlappingActor _array_element self :!class /Script/Engine.Actor)
        (if (not (Variables|Default|GetInteractionActive))
          (Variables|Default|SetInteractionActive true)
          (Class|BPIDialogue|Interact(Message) _array_element)
          (Components|Movement|StopMovementImmediately (Variables|Character|GetCharacterMovement))
          (else
            (Variables|Default|SetInteractionActive false)))))
    (if (not (Variables|Default|GetInteractionActive))
      ;[1 1 1] Move Character by clicking the location
      (Pawn|SetControlRotation (Game|GetPlayerController 0) (Math|Rotator|FindLookatRotation (Transformation|GetActorLocation (Game|GetPlayerCharacter 0)) (.location _hitresult)))
      (AI|Navigation|SimpleMovetoLocation (Game|GetPlayerController 0) (.location _hitresult)))))

(fn ConstructionScript)